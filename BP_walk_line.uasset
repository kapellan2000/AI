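; Spawner for a line of BP_CharLib characters that walk to points along a spline and later attack together.
; The construction script places Count-based target child actors along SplineTarget with random offsets and records their positions.
; Once a polled SpawnEvent flag is set, it spawns characters at intervals, passing those points plus randomized speed, delay, scale and end rotation.
; After a fire delay, it enables Attack on all characters sharing its ID tag.
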(event `self.ReceiveBeginPlay`
  (`KismetSystemLibrary.K2_SetTimerDelegate` (delegate `timer`) 0.01 true))

(event `timer`
  (bind _end_rotation_z__yaw_ (`self.End Rotation Z (Yaw)`))
  (bind _end_rotation_z__yaw_range (`self.End Rotation Z (Yaw)range`))
  (bind _speedrandomrange (`self.speedRandomRange`))
  (bind _startdelay_random (`self.StartDelay_random`))
  (if (`self.SpawnEvent`)
    (`/Engine/EditorBlueprintResources/StandardMacros.DoOnce` false
      (:`Completed`
        (if (>= (`self.Count`) 0) :!label _label
          (bind _returnvalue (`|SpawnActorFromClass` "/Game/AI/BP_CharLib.BP_CharLib_C" (`self.GetTransform` self) "AdjustIfPossibleButAlwaysSpawn" "OverrideRootScale" null null))
          (set `/Game/AI/BP_CharLib.attack` false _returnvalue)
          (`|ExecutionSequence`
            (:`then_0`
              (`KismetSystemLibrary.Delay` 0.2)
              (set `self.Count` (- (`self.Count`) 1))
              (goto _label))
            (:`then_1`
              (set `self.Spawned` _returnvalue)
              (set `/Game/AI/BP_CharLib.CharacterSK` (`self.Character`) (`self.Spawned`))
              (set `/Game/AI/BP_CharLib.Target` (`self.TargetPointSworm`) _returnvalue)
              (set `/Game/AI/BP_CharLib.Selection` "B" _returnvalue)
              (set `/Game/AI/BP_CharLib.EnemyDelay` (`self.Delay`) _returnvalue)
              (set `/Game/AI/BP_CharLib.FSpeed` (+ (`self.Speed`) (`KismetMathLibrary.RandomFloatInRange` (- 0.0 _speedrandomrange) _speedrandomrange)) _returnvalue)
              (set `/Game/AI/BP_CharLib.StartDelay` (+ (`self.startDelay`) (`KismetMathLibrary.RandomFloatInRange` (- 0.0 _startdelay_random) _startdelay_random)) _returnvalue)
              (set `/Game/AI/BP_CharLib.points` (`self.SplineCoord`) _returnvalue)
              (set `/Game/AI/BP_CharLib.Life` (`self.Count`) _returnvalue)
              (set `Actor.Tags` (`|MakeArray` (`self.ID`)) _returnvalue)
              (set `/Game/AI/BP_CharLib.EndRotation` (`KismetMathLibrary.MakeRotator` 0.0 0.0 (`KismetMathLibrary.RandomFloatInRange` (- _end_rotation_z__yaw_ _end_rotation_z__yaw_range) (+ _end_rotation_z__yaw_ _end_rotation_z__yaw_range))) _returnvalue)
              (set `/Game/AI/BP_CharLib.Scale` (`KismetMathLibrary.RandomFloatInRange` (`self.MinScale`) (`self.MaxScale`)) _returnvalue)
              (set `/Game/AI/BP_CharLib.capsuleRad` 0.1 _returnvalue)))
          (else
            (`KismetSystemLibrary.Delay` (`self.FireDelay`))
            (bind _outactors (`GameplayStatics.GetAllActorsWithTag` (`self.ID`)))
            (for _array_element _outactors
              (bind _asbp_char_lib (cast `/Game/AI/BP_CharLib` _array_element))
              (set `/Game/AI/BP_CharLib.attack` true _asbp_char_lib))))))))

(fn `NewFunction_0`)

(fn `UserConstructionScript`
  (bind _randendpos_x (`self.randEndPos_X`))
  (bind _randendpos_y (`self.randEndPos_Y`))
  (bind _splinetarget (`self.SplineTarget`))
  (bind _returnvalue (`SplineComponent.GetSplineLength` _splinetarget))
  (bind _childactors (`self.GetAllChildActors` self true))
  (`|ExecutionSequence`
    (:`then_0`
      ;[1 1 1] GoLine
      (if (> _returnvalue 100)
        (for _index (range (+ (`self.Count`) 1))
          (bind _returnvalue_2 (`AddComponent|NODE_AddChildActorComponent-6` :`RelativeTransform` (`KismetMathLibrary.MakeTransform` (`KismetMathLibrary.MakeVector` (+ (`KismetMathLibrary.RandomFloatInRange` (- 0.0 _randendpos_x) _randendpos_x) (.x (`SplineComponent.GetLocationAtDistanceAlongSpline` _splinetarget (* _index (/ (`KismetMathLibrary.Conv_FloatToDouble` _returnvalue) (`self.Count`))) "Local"))) (+ (`KismetMathLibrary.RandomFloatInRange` (- 0.0 _randendpos_y) _randendpos_y) (.y (`SplineComponent.GetLocationAtDistanceAlongSpline` _splinetarget (* _index (/ (`KismetMathLibrary.Conv_FloatToDouble` _returnvalue) (`self.Count`))) "Local")))))))
          (`ChildActorComponent.SetChildActorClass` _returnvalue_2 (`GameplayStatics.GetObjectClass` (`self.Target`)))
          (`KismetArrayLibrary.Array_Add` (`self.SplineCoord`) (`SceneComponent.K2_GetComponentLocation` _returnvalue_2)))))
    (:`then_1`
      ;[1 1 1] cast character
      (for (_ _array_index) _childactors
        (bind _asbp_char_lib (cast `/Game/AI/BP_CharLib` (`|GetArrayItem` _childactors _array_index)))
        (set `/Game/AI/BP_CharLib.CharacterSK` (`self.Character`) _asbp_char_lib)))))