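; Crowd spawner that places BP_CharLib characters in spline-based formations, for walking to targets or enemy-seeking.
; The construction script builds noisy row, staggered or triangle grids, either baked into SpawnPoint transforms or as child actors, with optional nav-point previews.
; With GoLine, it also stores shuffled destinations along SplineTarget.
; A looping timer waits for SpawnEvent, then spawns baked points once, passing each character movement, target, team-tag and life settings.
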(event `self.ReceiveBeginPlay`
  (`KismetSystemLibrary.K2_SetTimerDelegate` (delegate `Spawn`) 0.01 true))

(event `Spawn`
  (bind _spawned (`self.Spawned`))
  (bind _targetpointform (`self.TargetPointForm`))
  (if (`self.SpawnEvent`)
    (`/Engine/EditorBlueprintResources/StandardMacros.DoOnce` false
      (:`Completed`
        (for _array_element (`self.SpawnPoint`)
          (bind _returnvalue (`|SpawnActorFromClass` "/Game/AI/BP_CharLib.BP_CharLib_C" (`KismetMathLibrary.MakeTransform` (.location _array_element) (.rotation _array_element)) "AlwaysSpawn" "OverrideRootScale" null null))
          (set `self.Spawned` _returnvalue)
          (set `Actor.Tags` (`|MakeArray` (`self.TagName`)) _returnvalue)
          (set `self.counter` (+ (`self.counter`) 1))
          (set `/Game/AI/BP_CharLib.CharacterSK` (`self.Character`) (`self.Spawned`))
          ;[1 1 1] екфтіаук феек
          (set `/Game/AI/BP_CharLib.Scale` (`KismetMathLibrary.RandomFloatInRange` (`self.MaxScale`) (`self.MinScale`)) _spawned)
          (set `/Game/AI/BP_CharLib.SplineDot` (`|GetArrayItem` (`self.SplineCoord`) (`self.counter`)) _spawned)
          (`/Engine/EditorBlueprintResources/StandardMacros.IsValid` _targetpointform
            (:`Is Valid`
              (set `/Game/AI/BP_CharLib.endLocation` (`self.K2_GetActorLocation` _targetpointform) _spawned))
            (:`Is Not Valid`
              _))
          (set `/Game/AI/BP_CharLib.Target` (`self.TargetPointSworm`) _spawned)
          (set `/Game/AI/BP_CharLib.offset` (`SceneComponent.K2_GetComponentLocation` (`self.Spline`)) _spawned)
          (set `/Game/AI/BP_CharLib.FSpeed` (`self.Speed`) _spawned)
          (set `/Game/AI/BP_CharLib.SpeedRandom` (`self.SpeedRand`) _spawned)
          (set `/Game/AI/BP_CharLib.TargetOrSpline` (`self.GoLine`) _spawned)
          (set `/Game/AI/BP_CharLib.DegradateVec` (`self.Degradate(force,interval,delay start)`) _spawned)
          (set `/Game/AI/BP_CharLib.tagName` (`self.TagName`) _spawned)
          (set `/Game/AI/BP_CharLib.EnemyDelay` (`self.FindEnemyDelay`) _spawned)
          (set `/Game/AI/BP_CharLib.Life` (`self.SetLife`) _spawned)
          (set `/Game/AI/BP_CharLib.LRange` (`self.LongRange`) _spawned)
          (set `/Game/AI/BP_CharLib.HideBody` (`self.cremation`) _spawned)
          (set `/Game/AI/BP_CharLib.root` self _spawned)
          (set `/Game/AI/BP_CharLib.EndRotation` (`KismetMathLibrary.MakeRotator` 0.0 0.0 (`KismetMathLibrary.Conv_IntToDouble` (`self.AtacDirect`))) _spawned)
          (set `/Game/AI/BP_CharLib.EnemyTag` (`self.EnemyTag`) _spawned)
          (set `/Game/AI/BP_CharLib.StartDelay` (`self.FindEnemyDelay`) _spawned)
          (set `/Game/AI/BP_CharLib.AIFT` (`self.MoveByRoot`) _spawned)
          (set `/Game/AI/BP_CharLib.capsuleRad` (`self.capsule`) _spawned)
          (set `/Game/AI/BP_CharLib.offsetMove` (`self.Offset`) _spawned))))))

(fn `NewFunction_0`
  (bind _spacing (`self.Spacing`))
  (bind _spline (`self.Spline`))
  (bind _row (`self.row`))
  ;[1 1 1] ForwardRotation
  (set `self.CharCount` 0)
  (for _index (range (+ (`.ReturnValue` (`KismetMathLibrary.FMod` (`SplineComponent.GetSplineLength` _spline) _spacing)) 1))
    (for _index_2 (range (+ (select `bool` (`self.Triangle`) :`false` (select `bool` (and (> (`self.chess`) 0.0) (`KismetMathLibrary.Conv_IntToBool` (mod _index 2))) :`false` _row :`true` (- _row 1)) :`true` (- _row _index)) 1))
      (bind _returnvalue (* _index _spacing))
      (bind _returnvalue_2 (`KismetMathLibrary.MakeTransform` (`KismetMathLibrary.MakeVector` (.x (`SplineComponent.GetLocationAtDistanceAlongSpline` _spline _returnvalue "Local")) (+ (+ (`KismetMathLibrary.Conv_IntToDouble` (* _index_2 (`KismetMathLibrary.FTrunc` (`self.Spacing`)))) (.y (`SplineComponent.GetLocationAtDistanceAlongSpline` _spline _returnvalue "Local"))) (* (select `bool` (`self.Triangle`) :`false` (mod _index 2) :`true` _index) (`self.chess`))) (`self.ZLocation`)) (`SplineComponent.GetRotationAtDistanceAlongSpline` _spline _returnvalue "Local") (`KismetMathLibrary.Conv_DoubleToVector` (`KismetMathLibrary.RandomFloatInRange` (`self.MaxScale`) (`self.MinScale`)))))
      (bind _returnvalue_3 (`AddComponent|NODE_AddChildActorComponent-7` :`RelativeTransform` _returnvalue_2))
      (`|SpawnActorFromClass` "/Game/AI/BP_CharLib.BP_CharLib_C" _returnvalue_2 "Undefined" "OverrideRootScale" null null)))
  (`|ExecutionSequence`
    (:`then_0`
      (if true
        _))))

(fn `UserConstructionScript`
  (bind _startnoise (`self.StartNoise`))
  (bind _spline (`self.Spline`))
  (bind _linenoise (`self.LineNoise`))
  (bind _row (`self.row`))
  (bind _charcount (`self.CharCount`))
  (bind _splinetarget (`self.SplineTarget`))
  (bind _returnvalue (`SplineComponent.GetSplineLength` _splinetarget))
  (bind _childactors (`self.GetAllChildActors` self true))
  (bind _returnvalue_2 (* (`self.Spacing`) (`self.SpacingY`)))
  (bind _returnvalue_3 (* _linenoise -1.0))
  (bind _returnvalue_4 (`KismetMathLibrary.Conv_DoubleToVector` (`KismetMathLibrary.RandomFloatInRange` (`self.MaxScale`) (`self.MinScale`))))
  (if (not (`self.refresh`))
    ;[1 1 1] ForwardRotation
    (set `self.CharCount` 0)
    (for _index (range (+ (`.ReturnValue` (`KismetMathLibrary.FMod` (`SplineComponent.GetSplineLength` _spline) _returnvalue_2)) 1))
      (for _index_2 (range (+ (select `bool` (`self.Triangle`) :`false` (select `bool` (and (> (`self.chess`) 0.0) (`KismetMathLibrary.Conv_IntToBool` (mod _index 2))) :`false` _row :`true` (- _row 1)) :`true` (- _row _index)) 1))
        (if (`self.Bake`)
          (bind _returnvalue_5 (* _index _returnvalue_2))
          (bind _returnvalue_6 (`KismetMathLibrary.MakeTransform` (+ (`KismetMathLibrary.RandomPointInBoundingBox` (`KismetMathLibrary.MakeVector` (.x (`SplineComponent.GetLocationAtDistanceAlongSpline` _spline _returnvalue_5 "Local")) (+ (+ (`KismetMathLibrary.Conv_IntToDouble` (* _index_2 (`KismetMathLibrary.FTrunc` (`self.Spacing`)))) (.y (`SplineComponent.GetLocationAtDistanceAlongSpline` _spline _returnvalue_5 "Local"))) (* (select `bool` (`self.Triangle`) :`false` (mod _index 2) :`true` _index) (`self.chess`))) (`self.ZLocation`)) (`KismetMathLibrary.MakeVector` _startnoise _startnoise)) (`self.Offset`)) (`SplineComponent.GetRotationAtDistanceAlongSpline` _spline _returnvalue_5 "Local") _returnvalue_4))
          (`KismetArrayLibrary.Array_Add` (`self.SpawnPoint`) (`KismetMathLibrary.ComposeTransforms` _returnvalue_6 (`SceneComponent.K2_GetComponentToWorld` (`self.DefaultSceneRoot`))))
          (else
            (bind _returnvalue_7 (`AddComponent|NODE_AddChildActorComponent-0` :`RelativeTransform` _returnvalue_6))
            (`SceneComponent.SetWorldScale3D` _returnvalue_7 _returnvalue_4)
            (`ChildActorComponent.SetChildActorClass` _returnvalue_7 "/Game/AI/BP_CharLib.BP_CharLib_C")))
        (set `self.CharCount` (+ (`self.CharCount`) 1))
        (if (not (`self.HideNavPoint`))
          (bind _returnvalue_8 (`AddComponent|NODE_AddChildActorComponent-5` :`RelativeTransform` _returnvalue_6))
          (`SceneComponent.K2_SetWorldLocation` _returnvalue_8 (+ (`SceneComponent.K2_GetComponentLocation` (`Actor.RootComponent` (`self.TargetPointForm`))) (- (`SceneComponent.K2_GetComponentLocation` _returnvalue_8) (`SceneComponent.K2_GetComponentLocation` (`self.RootComponent`)))) false false)
          (`ChildActorComponent.SetChildActorClass` _returnvalue_8 (`GameplayStatics.GetObjectClass` (`self.TargetPointForm`))))))
    (`|ExecutionSequence`
      (:`then_0`
        (if (`self.GoLine`)
          ;[1 1 1] GoLine
          (if (> _returnvalue 100)
            (for _index_3 (range (+ _charcount 1))
              (bind _returnvalue_9 (`AddComponent|NODE_AddChildActorComponent-6` :`RelativeTransform` (`KismetMathLibrary.MakeTransform` (+ (`KismetMathLibrary.MakeVector` (.x (`SplineComponent.GetLocationAtDistanceAlongSpline` _splinetarget (* _index_3 (/ (`KismetMathLibrary.Conv_FloatToDouble` _returnvalue) _charcount)) "Local")) (.y (`SplineComponent.GetLocationAtDistanceAlongSpline` _splinetarget (* _index_3 (/ (`KismetMathLibrary.Conv_FloatToDouble` _returnvalue) _charcount)) "Local"))) (`KismetMathLibrary.MakeVector` (`KismetMathLibrary.RandomFloatInRangeFromStream` _returnvalue_3 _linenoise (`self.Stream`)) (`KismetMathLibrary.RandomFloatInRangeFromStream` _returnvalue_3 _linenoise (`self.Stream_0`)))))))
              (if (not (`self.HideNavPoint`))
                (`ChildActorComponent.SetChildActorClass` _returnvalue_9 (`GameplayStatics.GetObjectClass` (`self.TargetPointForm`))))
              (`KismetArrayLibrary.Array_Add` (`self.SplineCoord`) (`SceneComponent.K2_GetComponentLocation` _returnvalue_9)))
            (`KismetArrayLibrary.Array_Shuffle` (`self.SplineCoord`)))))
      (:`then_1`
        ;[1 1 1] cast character
        (for (_ _array_index) _childactors
          (bind _asbp_char_lib (cast `/Game/AI/BP_CharLib` (`|GetArrayItem` _childactors _array_index)))
          (set `/Game/AI/BP_CharLib.CharacterSK` (`self.Character`) _asbp_char_lib))))))