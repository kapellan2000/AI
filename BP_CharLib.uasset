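; Crowd-battle character that walks in formation or along waypoints and fights characters carrying its enemy tag, taking appearance from settings or a parent walk/stand box.
; Selection picks formation, target-actor path, point path or idle.
; Formation units shift with Root and blend destinations toward SplineDot as a timer raises Alpha.
; They seek tagged enemies, drain Life on overlap or randomly kill at long range; death disables collision and optionally sinks bodies.
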(event `distance`
  (bind _counter (`self.counter`))
  (bind _output (`|GetArrayItem` (`self.points`) _counter))
  (bind _returnvalue (+ _counter 1))
  ;[1 1 1] line
  (`CapsuleComponent.SetCapsuleRadius` (`self.CapsuleComponent`) 1.0 true)
  (if (< (`KismetMathLibrary.Vector_Distance` (`self.K2_GetActorLocation` self) _output) 300.0)
    (set `self.counter` _returnvalue :!label _label)
    (if (<= _returnvalue (+ (`self.Life`) 1))
      (`|AIMoveTo` self _output null
        (:`then`
          (set `CharacterMovementComponent.MaxWalkSpeed` (`self.FSpeed`) (`self.CharacterMovement`))
          (`KismetSystemLibrary.K2_SetTimerDelegate` (delegate `distance`) 0.01 true)))
      (else
        (`self.K2_SetActorRotation` (`self.EndRotation`))))))

(event `self.ReceiveBeginPlay`
  (bind _endlocation (`self.endLocation`))
  (bind _speedrandom (`self.SpeedRandom`))
  (bind _charactermovement (`self.CharacterMovement`))
  (bind _mesh (`self.Mesh`))
  (bind _target (`self.Target`))
  (bind _speedrandom_2 (`self.SpeedRandom`))
  (bind _fspeed (`self.FSpeed`))
  (bind _fspeed_2 (`self.FSpeed`))
  (bind _charactermovement_2 (`self.CharacterMovement`))
  (bind _enemytag (`self.EnemyTag`))
  (bind _counter (`self.counter`))
  (bind _returnvalue (+ _counter 1))
  (bind _returnvalue_2 (> (`self.alpha`) 1.0))
  (bind _returnvalue_3 (`KismetMathLibrary.RandomFloatInRange` (- _fspeed _speedrandom_2) (+ _fspeed _speedrandom_2)))
  (bind _returnvalue_4 (+ (- (`self.startLocation`) (`self.offset`)) _endlocation))
  (`KismetSystemLibrary.Delay` 1.0)
  (switch `string` (`self.Selection`)
    (:`Default`
      (`SceneComponent.K2_SetRelativeLocation` (`self.Mesh`) (`KismetMathLibrary.MakeVector` 0.0 0.0 (`self.Z`)) false false))
    (:`B`
      (set `CharacterMovementComponent.GravityScale` 100.0 (`self.CharacterMovement`))
      (`CapsuleComponent.SetCapsuleRadius` (`self.CapsuleComponent`) 5.0 true)))
  ;[1 1 1] setup char
  (`|ExecutionSequence`
    (:`then_0`
      (`SkinnedMeshComponent.SetSkinnedAssetAndUpdate` (`self.Mesh`) (`self.CharacterSK`) true)
      (`PrimitiveComponent.SetMaterial` _mesh 0 null)
      (`PrimitiveComponent.SetMaterial` _mesh 1 null)
      (`PrimitiveComponent.SetMaterial` _mesh 2 null)
      (`SceneComponent.SetWorldScale3D` (`self.Mesh`) (`KismetMathLibrary.Conv_DoubleToVector` (`self.Scale`)))
      (`CapsuleComponent.SetCapsuleRadius` (`self.CapsuleComponent`) (`self.capsuleRad`) true)
      (`SkinnedMeshComponent.SetSkinnedAssetAndUpdate` (`self.Mesh`) (`self.CharacterSK`) true)
      (set `self.startLocation` (`self.K2_GetActorLocation`))
      (switch `string` (`self.Selection`)
        (:`Default`
          ;[1 1 1] follow by start spline
          (set `self.rootInit` (`SceneComponent.K2_GetComponentLocation` (`/Game/AI/BP_walk_Box.DefaultSceneRoot` (`self.root`))))
          (`KismetSystemLibrary.K2_SetTimerDelegate` (delegate `animeteOffset`) 0.01 true)
          (set `self.rootStart` (`SceneComponent.K2_GetComponentLocation` (`/Game/AI/BP_walk_Box.DefaultSceneRoot` (`self.root`))))
          (`|ExecutionSequence`
            (:`then_0`
              (set `self.attack` false)
              ;[1 1 1] formation walk
              (if (`self.switch`)
                _
                (elif (== (0.0 0.0 0.0) _endlocation)
                  _
                  (elif (> (.x (`self.DegradateVec`)) 0.0)
                    (`KismetSystemLibrary.K2_SetTimerDelegate` (delegate `degradate`) (.y (`self.DegradateVec`)) (!= _returnvalue_2 true) (.z (`self.DegradateVec`)))
                    (if _returnvalue_2 :!label _label_2
                      (if (`self.TargetOrSpline`) :!label _label_3
                        (set `self.counter` (+ (`self.counter`) 1)))
                      (else
                        (if (`self.delay`) :!label _label_4
                          _
                          (elif (not (`self.attack`))
                            (`|AIMoveTo` self (`KismetMathLibrary.MakeVector` (.x (`KismetMathLibrary.VLerp` _returnvalue_4 (`KismetMathLibrary.MakeVector` (.x (`self.SplineDot`)) (.y (`self.SplineDot`)) (.z _returnvalue_4)) (`self.alpha`))) (.y (`KismetMathLibrary.VLerp` _returnvalue_4 (`KismetMathLibrary.MakeVector` (.x (`self.SplineDot`)) (.y (`self.SplineDot`)) (.z _returnvalue_4)) (`self.alpha`))) 2220.0) null 100.0 true
                              (:`then`
                                (if (> (`self.alpha`) 0.5)
                                  (set `CharacterMovementComponent.MaxWalkSpeed` (`KismetMathLibrary.RandomFloatInRange` (- _fspeed_2 _speedrandom) (+ _fspeed_2 _speedrandom)) _charactermovement)
                                  (else
                                    (set `CharacterMovementComponent.MaxWalkSpeed` _fspeed_2 _charactermovement))))
                              (:`OnSuccess`
                                (goto _label_3))
                              (:`OnFail`))))))
                    (else
                      (goto _label_4))))))
            (:`then_1`
              ;[1 1 1] AI FIND TARGET
              (`KismetSystemLibrary.K2_SetTimerDelegate` (delegate `Finder`) 0.2 false (`self.StartDelay`))
              ;[1 1 1] long range
              (if (`self.LRange`)
                (bind _outactors (`GameplayStatics.GetAllActorsWithTag` (select `bool` (!= _enemytag (`self.tagName`)) :`false` (`self.tagName`) :`true` _enemytag)))
                (`KismetSystemLibrary.K2_SetTimerDelegate` (delegate `LRangeTimer`) 1.0 true)))))
        (:`A`
          ;[1 1 1] byPoint
          (`KismetSystemLibrary.Delay` (`self.StartDelay`))
          (set `self.counter` _returnvalue :!label _label_5)
          (if (<= _returnvalue (`KismetArrayLibrary.Array_Length` _target))
            (`|AIMoveTo` self (`self.K2_GetActorLocation` (`|GetArrayItem` _target _counter)) null
              (:`then`
                (set `CharacterMovementComponent.MaxWalkSpeed` _returnvalue_3 _charactermovement_2))
              (:`OnSuccess`
                (set `CharacterMovementComponent.MaxWalkSpeed` _returnvalue_3 _charactermovement_2)
                (`KismetSystemLibrary.Delay` (`self.EnemyDelay`))
                (goto _label_5)))))
        (:`B`
          (goto _label))
        (:`C`
          (`CapsuleComponent.SetCapsuleRadius` (`self.CapsuleComponent`) 1.0 true)
          (set `CharacterMovementComponent.MaxWalkSpeed` 0.0 (`self.CharacterMovement`))
          (set `self.attack` false))))))

(event `degradate`
  ;[1 1 1] formation walk
  (set `self.alpha` (+ (`self.alpha`) (/ (.x (`self.DegradateVec`)) 100.0)))
  (goto _label_2))

(event `animeteOffset`
  (bind _root (`self.root`))
  (bind _returnvalue (`SceneComponent.K2_GetComponentLocation` (`/Game/AI/BP_walk_Box.DefaultSceneRoot` (`self.root`))))
  ;[1 1 1] follow by start spline
  ;[1 1 1] move by root
  (if (`self.AIFT`)
    (`self.K2_SetActorLocation` (select `bool` (== (`self.alpha`) 0.0) :`false` (+ (- _returnvalue (`self.rootStart`)) (`self.K2_GetActorLocation` self)) :`true` (+ (- (`SceneComponent.K2_GetComponentLocation` (`/Game/AI/BP_walk_Box.DefaultSceneRoot` _root)) (`self.rootInit`)) (`self.startLocation`))))
    (set `self.rootStart` _returnvalue)
    (`SceneComponent.SetVisibility` (`self.Mesh`) (`/Game/AI/BP_walk_Box.visibility` _root) false)))

(event `self.Cube.OnComponentBeginOverlap`
  (params (OverlappedComponent :type "PrimitiveComponent Object Reference") (OtherActor :type "Actor Object Reference") (OtherComp :type "PrimitiveComponent Object Reference") (OtherBodyIndex :type Integer) (bFromSweep :type Boolean) (SweepResult :type "HitResult Structure (by ref)"))
  (bind _returnvalue (* (`self.capsuleRad`) 3.0))
  ;[1 1 1] atac
  (switch `string` (`self.Selection`)
    (:`Default`
      (if (not (`self.attack`))
        (bind _asbp_char_lib (cast `/BP_CharLib` OtherActor))
        (if (== (`/BP_CharLib.tagName` _asbp_char_lib) (`self.EnemyTag`))
          (`CapsuleComponent.SetCapsuleSize` (`self.CapsuleComponent`) _returnvalue _returnvalue true)
          (set `self.attack` true)
          (`KismetSystemLibrary.K2_SetTimerDelegate` (delegate `AtacTick`) 2.0 true))))))

(event `AtacTick`
  (bind _capsulecomponent (`self.CapsuleComponent`))
  ;[1 1 1] atac
  (if (`self.attack`)
    (set `/BP_CharLib.Life` (- (`/BP_CharLib.Life` (stale `self.Cube.OnComponentBeginOverlap` _asbp_char_lib)) 1) (stale `self.Cube.OnComponentBeginOverlap` _asbp_char_lib))
    (`|ExecutionSequence`
      (:`then_1`
        (if (< (`self.Life`) 1)
          (switch `string` (`self.Selection`) :!label _label_6
            (:`Default`
              ;[1 1 1] kill
              (set `self.Dead` true)
              (`SceneComponent.K2_SetRelativeLocation` (`self.Cube`) (0.0 0.0 -400.0) false false)
              (`PrimitiveComponent.SetCollisionEnabled` (`self.CapsuleComponent`) "NoCollision")
              (if (`self.HideBody`)
                (`KismetSystemLibrary.Delay` 5.0)
                (`SceneComponent.K2_SetRelativeLocation` (`self.Mesh`) (0.0 0.0 -400.0) false false)
                (`SceneComponent.K2_SetRelativeLocation` (`self.CapsuleComponent`) (0.0 0.0 -400.0) false false)))))))
    (else
      ;[1 1 1] after fight
      (set `self.attack` false)
      (if (`self.done`)
        _
        (elif (not (`self.Dead`))
          (`|AIMoveTo` null (`KismetMathLibrary.MakeVector` (.x (`self.SplineDot`)) (.y (`self.SplineDot`)) 2220.0) null 10.0 true
            (:`then`
              (if (< (`KismetMathLibrary.VSize` (`self.GetVelocity` self)) 50.0)
                _))
            (:`OnSuccess`
              (set `self.done` true))
            (:`OnFail`
              (`CapsuleComponent.SetCapsuleRadius` _capsulecomponent (* (`self.capsuleRad`) 1.3) true)
              (`KismetSystemLibrary.Delay` 1.0)
              (`CapsuleComponent.SetCapsuleRadius` _capsulecomponent (`self.capsuleRad`) true))))))))

(event `Finder`
  ;[1 1 1] AI FIND TARGET
  (if (`self.attack`) :!label _label_7
    _
    (elif (not (`self.Dead`))
      (bind _outactors (`GameplayStatics.GetAllActorsWithTag` (`self.EnemyTag`)))
      (if (> (`KismetArrayLibrary.Array_Length` _outactors) 0)
        (if (< (`KismetMathLibrary.VSize` (`self.GetVelocity` self)) 100.0)
          (bind _outitem (`KismetArrayLibrary.Array_Random` _outactors))
          (`|AIMoveTo` self (`KismetMathLibrary.MakeVector` (.x (`self.K2_GetActorLocation` _outitem)) (.y (`self.K2_GetActorLocation` _outitem)) 2220.0) _outitem 5.0 true
            (:`OnSuccess`
              (`KismetSystemLibrary.Delay` 1.0)
              (goto _label_7)))
          (else
            (bind (_distance _returnvalue) (`GameplayStatics.FindNearestActor` (`self.K2_GetActorLocation` self) _outactors))
            (`|AIMoveTo` self (`KismetMathLibrary.MakeVector` (.x (`self.K2_GetActorLocation` _returnvalue)) (.y (`self.K2_GetActorLocation` _returnvalue)) 2220.0) _returnvalue 5.0 true
              (:`OnSuccess`
                (`KismetSystemLibrary.Delay` 2.0)
                (goto _label_7)))))))))

(event `LRangeTimer`
  ;[1 1 1] long range
  (bind (_distance _returnvalue) (`GameplayStatics.FindNearestActor` (`self.K2_GetActorLocation` self) (stale `self.ReceiveBeginPlay` _outactors)))
  (if (< _distance 10000.0)
    (`|ExecutionSequence`
      (:`then_0`
        (if (`KismetMathLibrary.RandomBoolWithWeight` 0.05)
          (bind _asbp_char_lib (cast `/BP_CharLib` _returnvalue))
          (set `/BP_CharLib.Life` 0 _asbp_char_lib)
          (set `/BP_CharLib.attack` false _asbp_char_lib)
          (set `/BP_CharLib.Dead` true _asbp_char_lib)
          (`|AIMoveTo` _asbp_char_lib (0.0 0.0 0.0) _asbp_char_lib 100.0 true
            (:`then`
              (`SceneComponent.K2_SetRelativeLocation` (`/BP_CharLib.Cube` _asbp_char_lib) (0.0 0.0 -400.0) false false)
              (bind _capsulecomponent (`Character.CapsuleComponent` _asbp_char_lib))
              (`PrimitiveComponent.SetCollisionEnabled` _capsulecomponent "NoCollision")
              (if (`self.HideBody`)
                (`KismetSystemLibrary.Delay` 5.0)
                (`SceneComponent.K2_SetRelativeLocation` _capsulecomponent (0.0 0.0 -400.0) false false))))))
      (:`then_1`
        (`|AIMoveTo` self (`self.K2_GetActorLocation` self) null 100.0 true
          (:`then`
            _)
          (:`OnSuccess`
            _)
          (:`OnFail`
            _))
        (if (`self.Dead`)
          _
          (elif (< (`self.Life`) 1)
            (set `self.attack` false)
            (goto _label_6)
            (else
              (set `self.attack` true)
              (`self.K2_SetActorRotation` self (`KismetMathLibrary.FindLookAtRotation` (`self.K2_GetActorLocation` self) (`self.K2_GetActorLocation` _returnvalue)) false))))))
    (else
      (set `self.attack` false))))

(fn `UserConstructionScript`
  (bind _returnvalue (`self.GetParentActor`))
  (bind _mesh (`self.Mesh`))
  (bind _mesh_2 (`self.Mesh`))
  (bind _asbp_walk_box (cast `/Game/AI/BP_walk_Box` _returnvalue)
    (:`then`
      (`PrimitiveComponent.SetMaterial` _mesh_2 0 null)
      (`PrimitiveComponent.SetMaterial` _mesh_2 1 null)
      (`PrimitiveComponent.SetMaterial` _mesh_2 2 null)
      (`SkinnedMeshComponent.SetSkinnedAssetAndUpdate` _mesh_2 (`/Game/AI/BP_walk_Box.Character` _asbp_walk_box) true)
      (`CapsuleComponent.SetCapsuleRadius` (`self.CapsuleComponent`) (`/Game/AI/BP_walk_Box.capsule` _asbp_walk_box) true))
    (:`CastFailed`
      (bind _asbp_stand_box (cast `/Game/AI/BP_stand_Box` _returnvalue))
      (`PrimitiveComponent.SetMaterial` _mesh 0 null)
      (`PrimitiveComponent.SetMaterial` _mesh 1 null)
      (`PrimitiveComponent.SetMaterial` _mesh 2 null)
      (`SkinnedMeshComponent.SetSkinnedAssetAndUpdate` _mesh (`/Game/AI/BP_stand_Box.Character` _asbp_stand_box) true))))