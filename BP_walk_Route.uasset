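; BP_walk_Route is a route actor that spawns one BP_CharLib walking character at its own transform on BeginPlay.
; It passes the character its mesh, target point, speed and delay settings, with selection fixed to "A".
; With Refresh off, construction adds a classless child actor component at the SplineTarget start, records its location and updates child characters' mesh.
; Spline-based crowd scattering remains as disconnected, unused logic.
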(event `self.ReceiveBeginPlay`
  (bind _returnvalue (`|SpawnActorFromClass` "/Game/AI/BP_CharLib.BP_CharLib_C" (`self.GetTransform` self) "AlwaysSpawn" "OverrideRootScale" null null))
  (set `self.Spawned` _returnvalue)
  (set `/Game/AI/BP_CharLib.CharacterSK` (`self.Character`) (`self.Spawned`))
  (set `/Game/AI/BP_CharLib.Target` (`self.TargetPointSworm`) _returnvalue)
  (set `/Game/AI/BP_CharLib.Selection` "A" _returnvalue)
  (set `/Game/AI/BP_CharLib.EnemyDelay` (`self.Delay`) _returnvalue)
  (set `/Game/AI/BP_CharLib.FSpeed` (`self.Speed`) _returnvalue)
  (set `/Game/AI/BP_CharLib.SpeedRandom` (`self.SpeedRand`) _returnvalue)
  (set `/Game/AI/BP_CharLib.StartDelay` (`self.startDelay`) _returnvalue))

(fn `NewFunction_0`)

(fn `UserConstructionScript`
  (bind _splinetarget (`self.SplineTarget`))
  (bind _returnvalue (`SplineComponent.GetSplineLength` _splinetarget))
  (bind _childactors (`self.GetAllChildActors` self true))
  (if (not (`self.refresh`))
    (`|ExecutionSequence`
      (:`then_0`
        (if true
          ;[1 1 1] GoLine
          (if (> _returnvalue 100)
            (`KismetSystemLibrary.PrintString` (`KismetStringLibrary.Conv_DoubleToString` _returnvalue))
            (for _index (range 1)
              (bind _returnvalue_2 (`AddComponent|NODE_AddChildActorComponent-6` :`RelativeTransform` (`KismetMathLibrary.MakeTransform` (+ (`KismetMathLibrary.MakeVector` (.x (`SplineComponent.GetLocationAtDistanceAlongSpline` _splinetarget (* _index (/ (`KismetMathLibrary.Conv_FloatToDouble` _returnvalue) 0.0)) "Local")) (.y (`SplineComponent.GetLocationAtDistanceAlongSpline` _splinetarget (* _index (/ (`KismetMathLibrary.Conv_FloatToDouble` _returnvalue) 0.0)) "Local"))) (0.0 0.0 0.0)))))
              (if (not true)
                (`ChildActorComponent.SetChildActorClass` _returnvalue_2 null))
              (`KismetArrayLibrary.Array_Add` (`self.SplineCoord`) (`SceneComponent.K2_GetComponentLocation` _returnvalue_2))))))
      (:`then_1`
        ;[1 1 1] cast character
        (for (_ _array_index) _childactors
          (bind _asbp_char_lib (cast `/Game/AI/BP_CharLib` (`|GetArrayItem` _childactors _array_index)))
          (set `/Game/AI/BP_CharLib.CharacterSK` (`self.Character`) _asbp_char_lib))))))