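; Formation spawner that lays out a crowd of BP_CharLib characters along a spline in rows, with triangle or staggered layout, position noise and random scale.
; The construction script, skipped when Refresh is set, either bakes world transforms into SpawnPoint or adds child actors directly.
; At play, a self-looping chain spawns from SpawnPoint instantly, delayed, shuffled or row-paced per Pattern, tags each character with ID, then triggers their Attack after DelayFire.
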(event `self.ReceiveBeginPlay`
  (`KismetSystemLibrary.K2_SetTimerDelegate` (delegate `Spawn`) 0.01 true))

(event `Spawn`
  (bind _spawned (`self.Spawned`))
  (bind _spawnpoint (`self.SpawnPoint`))
  (bind _returnvalue (/ (`self.counter`) (+ (`self.row`) 1)))
  (`/Engine/EditorBlueprintResources/StandardMacros.DoOnce` false
    (:`Completed`
      (if (<= (`KismetArrayLibrary.Array_Length` (`self.SpawnPoint`)) (`self.counter`)) :!label _label
        (`KismetSystemLibrary.Delay` (`self.DelayFire`))
        (bind _outactors (`GameplayStatics.GetAllActorsWithTag` (`self.ID`)))
        (for _array_element _outactors
          (bind _asbp_char_lib (cast `/Game/AI/BP_CharLib` _array_element))
          (set `/Game/AI/BP_CharLib.attack` true _asbp_char_lib))
        (else
          (switch `int` (`self.pattern`)
            (:`0`
              (bind _returnvalue_2 (`|SpawnActorFromClass` "/Game/AI/BP_CharLib.BP_CharLib_C" (`KismetMathLibrary.MakeTransform` (.location (`|GetArrayItem` _spawnpoint (`self.counter`))) (.rotation (`|GetArrayItem` _spawnpoint (`self.counter`)))) "AlwaysSpawn" "OverrideRootScale" null null :!label _label_2))
              (set `self.Spawned` _returnvalue_2)
              (set `Actor.Tags` (`|MakeArray` (`self.ID`)) _returnvalue_2)
              (set `self.counter` (+ (`self.counter`) 1))
              (set `/Game/AI/BP_CharLib.CharacterSK` (`self.Character`) (`self.Spawned`))
              ;[1 1 1] екфтіаук феек
              (set `/Game/AI/BP_CharLib.Scale` (`KismetMathLibrary.RandomFloatInRange` (`self.MaxScale`) (`self.MinScale`)) _spawned)
              (set `/Game/AI/BP_CharLib.Selection` "C" _spawned)
              (`SceneComponent.SetVisibility` (`Character.Mesh` _spawned) false false)
              (`SceneComponent.SetVisibility` (`Actor.RootComponent` _spawned) true false)
              (`SceneComponent.SetVisibility` (`Character.Mesh` _spawned) true false)
              (set `/Game/AI/BP_CharLib.tagName` (`self.ID`) _spawned)
              (goto _label))
            (:`1`
              (`KismetSystemLibrary.Delay` (`self.SpawnDelay`) :!label _label_3)
              (goto _label_2))
            (:`2`
              (`|ExecutionSequence`
                (:`then_0`
                  (goto _label_3))
                (:`then_1`
                  (`/Engine/EditorBlueprintResources/StandardMacros.DoOnce` false
                    (:`Completed`
                      (`KismetArrayLibrary.Array_Shuffle` _spawnpoint))))))
            (:`3`
              (if (!= _returnvalue (`self.rowCounter`))
                (set `self.rowCounter` _returnvalue)
                (`KismetSystemLibrary.Delay` (`self.SpawnDelay`))
                (goto _label_2)
                (else
                  (goto _label_2))))))))))

(fn `NewFunction_0`
  (bind _spacing (`self.Spacing`))
  (bind _spline (`self.Spline`))
  (bind _row (`self.row`))
  ;[1 1 1] ForwardRotation
  (set `self.CharCount` 0)
  (for _index (range (+ (`.ReturnValue` (`KismetMathLibrary.FMod` (`SplineComponent.GetSplineLength` _spline) _spacing)) 1))
    (for _index_2 (range (+ (select `bool` (`self.Triangle`) :`false` (select `bool` (and (> (`self.chess`) 0.0) (`KismetMathLibrary.Conv_IntToBool` (mod _index 2))) :`false` _row :`true` (- _row 1)) :`true` (- _row _index)) 1))
      (bind _returnvalue (* _index _spacing))
      (bind _returnvalue_2 (`KismetMathLibrary.MakeTransform` (`KismetMathLibrary.MakeVector` (.x (`SplineComponent.GetLocationAtDistanceAlongSpline` _spline _returnvalue "Local")) (+ (+ (`KismetMathLibrary.Conv_IntToDouble` (* _index_2 (`KismetMathLibrary.FTrunc` (`self.Spacing`)))) (.y (`SplineComponent.GetLocationAtDistanceAlongSpline` _spline _returnvalue "Local"))) (* (select `bool` (`self.Triangle`) :`false` (mod _index 2) :`true` _index) (`self.chess`))) 0.0) (`SplineComponent.GetRotationAtDistanceAlongSpline` _spline _returnvalue "Local") (`KismetMathLibrary.Conv_DoubleToVector` (`KismetMathLibrary.RandomFloatInRange` (`self.MaxScale`) (`self.MinScale`)))))
      (bind _returnvalue_3 (`AddComponent|NODE_AddChildActorComponent-7` :`RelativeTransform` _returnvalue_2))
      (`|SpawnActorFromClass` "/Game/AI/BP_CharLib.BP_CharLib_C" _returnvalue_2 "Undefined" "OverrideRootScale" null null)))
  (`|ExecutionSequence`
    (:`then_0`
      (if true
        _))))

(fn `UserConstructionScript`
  (bind _startnoise (`self.StartNoise`))
  (bind _spline (`self.Spline`))
  (bind _row (`self.row`))
  (bind _childactors (`self.GetAllChildActors` self true))
  (bind _returnvalue (* (`self.Spacing`) (`self.SpacingY`)))
  (bind (_remainder _returnvalue_2) (`KismetMathLibrary.FMod` (`SplineComponent.GetSplineLength` _spline) _returnvalue))
  (bind _returnvalue_3 (`KismetMathLibrary.Conv_DoubleToVector` (`KismetMathLibrary.RandomFloatInRange` (`self.MaxScale`) (`self.MinScale`))))
  (if (not (`self.refresh`))
    ;[1 1 1] ForwardRotation
    (set `self.CharCount` 0)
    (set `self.cell` _returnvalue_2)
    (for _index (range (+ _returnvalue_2 1))
      (for _index_2 (range (+ (select `bool` (`self.Triangle`) :`false` (select `bool` (and (> (`self.chess`) 0.0) (`KismetMathLibrary.Conv_IntToBool` (mod _index 2))) :`false` _row :`true` (- _row 1)) :`true` (- _row _index)) 1))
        (if (`self.Bake`)
          (bind _returnvalue_4 (* _index _returnvalue))
          (bind _returnvalue_5 (`KismetMathLibrary.MakeTransform` (+ (`KismetMathLibrary.RandomPointInBoundingBox` (`KismetMathLibrary.MakeVector` (.x (`SplineComponent.GetLocationAtDistanceAlongSpline` _spline _returnvalue_4 "Local")) (+ (+ (`KismetMathLibrary.Conv_IntToDouble` (* _index_2 (`KismetMathLibrary.FTrunc` (`self.Spacing`)))) (.y (`SplineComponent.GetLocationAtDistanceAlongSpline` _spline _returnvalue_4 "Local"))) (* (select `bool` (`self.Triangle`) :`false` (mod _index 2) :`true` _index) (`self.chess`))) 0.0) (`KismetMathLibrary.MakeVector` _startnoise _startnoise)) (0.0 0.0 0.0)) (`KismetMathLibrary.MakeRotator` (.roll (`SplineComponent.GetRotationAtDistanceAlongSpline` _spline _returnvalue_4 "Local")) (.pitch (`SplineComponent.GetRotationAtDistanceAlongSpline` _spline _returnvalue_4 "Local")) (`self.Orient`)) _returnvalue_3))
          (`KismetArrayLibrary.Array_Add` (`self.SpawnPoint`) (`KismetMathLibrary.ComposeTransforms` _returnvalue_5 (`SceneComponent.K2_GetComponentToWorld` (`self.DefaultSceneRoot`))))
          (else
            (bind _returnvalue_6 (`AddComponent|NODE_AddChildActorComponent-0` :`RelativeTransform` _returnvalue_5))
            (`SceneComponent.SetWorldScale3D` _returnvalue_6 _returnvalue_3)
            (`ChildActorComponent.SetChildActorClass` _returnvalue_6 "/Game/AI/BP_CharLib.BP_CharLib_C")))
        (set `self.CharCount` (+ (`self.CharCount`) 1))))
    (`|ExecutionSequence`
      (:`then_1`
        ;[1 1 1] cast character
        (for (_ _array_index) _childactors
          (bind _asbp_char_lib (cast `/Game/AI/BP_CharLib` (`|GetArrayItem` _childactors _array_index)))
          (set `/Game/AI/BP_CharLib.CharacterSK` (`self.Character`) _asbp_char_lib))))))